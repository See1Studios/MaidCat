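; Projector actor that supplies a texture, color and projection settings (perspective or orthographic) to a Niagara system and to materials.
; When shadows are enabled, its construction script adds a downward-pitched depth scene capture rendering to a low-resolution R16f target sized by aspect.
; The construction script then pushes all settings and that shadow target to Niagara.
; SetProjectorParameters writes similar values to a given material, with PerspectiveEnabled fixed at 0.
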(fn `SetNiagaraVariables`
  (bind _niagara (`self.Niagara`))
  (bind _niagara_2 (`self.Niagara`))
  (bind _niagara_3 (`self.Niagara`))
  (`NiagaraComponent.SetVariableTexture` _niagara "Texture" (`self.Texture`))
  (`NiagaraComponent.SetVariableTextureRenderTarget` _niagara "ShadowRT" (select `bool` (`self.ShadowEnabled`) :`true` (`self.ShadowRT`) :!type "TextureRenderTarget Object Reference"))
  (`NiagaraComponent.SetVariableLinearColor` _niagara "Color" (`self.Color`))
  (`NiagaraComponent.SetVariableFloat` _niagara "Aspect" (`self.Aspect`))
  (`NiagaraComponent.SetVariableFloat` _niagara "Near" (`self.Near`))
  (`NiagaraComponent.SetVariableFloat` _niagara_2 "Far" (`self.Far`))
  (`NiagaraComponent.SetVariableFloat` _niagara_2 "OrthoWidth" (`self.OrthoWidth`))
  (`NiagaraComponent.SetVariableFloat` _niagara_2 "Perspective" (select `ECameraProjectionMode` (`self.ProjectionType`) :`Perspective` 1.0 :!type "Float (single-precision)"))
  (`NiagaraComponent.SetVariableFloat` _niagara_3 "FOV" (`self.FOV`))
  (`NiagaraComponent.SetVariableFloat` _niagara_3 "FocalDistance" (`self.FocalDistance`))
  (`NiagaraComponent.SetVariableFloat` _niagara_3 "ShadowEnabled" (`KismetMathLibrary.SelectFloat` 1.0 0.0 (`self.ShadowEnabled`))))

(fn `SetProjectorParameters`
  (params (Material :type "MaterialInstanceDynamic Object Reference"))
  (locals (mat :type "MaterialInstanceDynamic Object Reference"))
  (bind _mat (`local.mat`))
  (bind _mat_2 (`local.mat`))
  (set `local.mat` Material)
  (`MaterialInstanceDynamic.SetScalarParameterValue` _mat "Aspect" (`self.Aspect`))
  (`MaterialInstanceDynamic.SetScalarParameterValue` _mat "Near" (`self.Near`))
  (`MaterialInstanceDynamic.SetScalarParameterValue` _mat "Far" (`self.Far`))
  (`MaterialInstanceDynamic.SetScalarParameterValue` _mat "PerspectiveEnabled" (`KismetMathLibrary.SelectFloat` 1.0))
  (`MaterialInstanceDynamic.SetScalarParameterValue` _mat "FOV" (`self.FOV`))
  (`MaterialInstanceDynamic.SetScalarParameterValue` _mat "OrthoWidth" (`self.OrthoWidth`))
  (`MaterialInstanceDynamic.SetTextureParameterValue` _mat_2 "Texture" (`self.Texture`))
  (`MaterialInstanceDynamic.SetTextureParameterValue` _mat_2 "ShadowRT" (`self.ShadowRT`))
  (`MaterialInstanceDynamic.SetVectorParameterValue` _mat_2 "Color" (`self.Color`)))

(fn `UserConstructionScript`
  (bind _scenecapture (`self.SceneCapture`))
  (`|ExecutionSequence`
    (:`then_0`
      (if (`self.ShadowEnabled`)
        (`|ExecutionSequence`
          (:`then_0`
            (bind _returnvalue (`AddComponent|NODE_AddSceneCaptureComponent2D-1` :`RelativeTransform` (`KismetMathLibrary.MakeTransform` (0.0 0.0 0.0) (struct :`Roll` -90.0))))
            (set `self.SceneCapture` _returnvalue))
          (:`then_1`
            (set `SceneCaptureComponent.CaptureSource` "SCS_SceneDepth" _scenecapture)
            (set `SceneCaptureComponent2D.FOVAngle` (`self.FOV`) _scenecapture)
            (set `SceneCaptureComponent2D.ProjectionType` (`self.ProjectionType`) _scenecapture)
            (set `SceneCaptureComponent2D.OrthoWidth` (`self.OrthoWidth`) _scenecapture))
          (:`then_2`
            (bind _returnvalue_2 (`KismetRenderingLibrary.CreateRenderTarget2D` (`KismetMathLibrary.Round` (* (`self.Aspect`) 128)) 128 "RTF_R16f" (struct :`A` 1.0) true))
            (bind _output_get (set `self.ShadowRT` _returnvalue_2))
            (set `SceneCaptureComponent2D.TextureTarget` _output_get (`self.SceneCapture`))))))
    (:`then_1`
      (`self.SetNiagaraVariables`))))