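; Blueprint function library of helper utilities for the MaidCat plugin.
; GetMaidCatDir returns the plugin's base directory and its Python subfolder.
; CollectMaterials walks the primitive components of given actors and gathers unique base Materials, resolving material instances one parent level up, so nested instance chains are skipped.
; FilterEngineContents returns the given objects without those whose path contains "/Engine".
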(fn `CollectMaterials`
  (params (Actors :type "Array of Actor Object Reference"))
  (returns (Materials :type "Array of Material Object Reference"))
  (locals (_materials :type "Array of Material Object Reference"))
  (`|ExecutionSequence`
    (:`then_0`
      (for _array_element Actors
        (for _array_element_2 (`Actor.K2_GetComponentsByClass` _array_element "/Script/Engine.PrimitiveComponent")
          (for _index (range (+ (`PrimitiveComponent.GetNumMaterials` _array_element_2) 1))
            (bind _returnvalue (`PrimitiveComponent.GetMaterial` _array_element_2 _index))
            (bind `_as머티리얼_인스턴스` (cast `MaterialInstance` _returnvalue)
              (:`then`
                (bind `_as머티리얼` (cast `Material` (`MaterialInstance.Parent` `_as머티리얼_인스턴스`)))
                (`KismetArrayLibrary.Array_AddUnique` (`local._materials`) `_as머티리얼`))
              (:`CastFailed`
                (bind `_as머티리얼_2` (cast `Material` _returnvalue))
                (`KismetArrayLibrary.Array_AddUnique` (`local._materials`) `_as머티리얼_2`)))))))
    (:`then_1`
      (return (`local._materials`)))))

(fn `FilterEngineContents`
  (params (Objects :type "Array of Object Object Reference"))
  (returns (Result :type "Array of Object Object Reference"))
  (locals (temp :type "Array of Object Object Reference"))
  (for _array_element Objects
    (if (not (`KismetStringLibrary.Contains` (`KismetSystemLibrary.GetPathName` _array_element) "/Engine" true))
      (`KismetArrayLibrary.Array_AddUnique` (`local.temp`) _array_element)))
  (return (`local.temp`)))

(fn `GetMaidCatDir`
  (returns (SystemPath :type String) (PythonPath :type String))
  (bind _outbasedir (`PluginBlueprintLibrary.GetPluginBaseDir` "MaidCat"))
  (return _outbasedir (`KismetStringLibrary.Concat_StrStr` _outbasedir "Python/")))